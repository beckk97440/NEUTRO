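; Elevator button that lowers a referenced elevator actor when its UseElevator event fires.
; The construction script caches the elevator's start location.
; A timeline then lerps the elevator from that point down the Z axis by the Etage distance, without sweeping.
; The timeline only plays forward, so this graph has no return trip.
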(event `UseElevator`
  (bind (_direction _alpha) (`Timeline|Elevator_Timeline`)
    (:`Update`
      (`self.K2_SetActorLocation` (`self.ElevatorRef`) (`KismetMathLibrary.VLerp` (`self.StartElevatorLocation`) (- (`self.StartElevatorLocation`) (`KismetMathLibrary.MakeVector` 0.0 0.0 (`self.Etage?`))) _alpha) false false))))

(fn `UserConstructionScript`
  (set `self.StartElevatorLocation` (`self.K2_GetActorLocation` (`self.ElevatorRef`))))