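; Automatic double sliding door that can be locked by a padlock actor.
; A box trigger detects the tagged player capsule, playing the Mover timeline to slide both meshes along relative Y, then reversing it after a short delay on exit.
; While locked (Verrouiller), Tick watches the padlock reference (CadenasRef); once it becomes invalid, the door opens once and unlocks for normal trigger use.
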(event `self.ReceiveTick`
  (params (DeltaSeconds :type "Float (single-precision)"))
  ;[1 1 1] Event Tick
  (if (`self.Verrouiller`)
    (`/Engine/EditorBlueprintResources/StandardMacros.IsValid` (`self.Cadenas_Ref`)
      (:`Is Not Valid`
        (`/Engine/EditorBlueprintResources/StandardMacros.DoOnce` false
          (:`Completed`
            (`self.1`)
            (set `self.Verrouiller` false)))))))

(event `self.ReceiveBeginPlay`
  ;[1 1 1] Event Begin Play
  (set `self.Door1StartLocation` (`SceneComponent.K2_GetComponentLocation` (`self.StaticMesh`)))
  (set `self.Door2StartLocation` (`SceneComponent.K2_GetComponentLocation` (`self.StaticMesh1`))))

(event `self.BoxTrigger.OnComponentBeginOverlap`
  (params (OverlappedComponent :type "PrimitiveComponent Object Reference") (OtherActor :type "Actor Object Reference") (OtherComp :type "PrimitiveComponent Object Reference") (OtherBodyIndex :type Integer) (bFromSweep :type Boolean) (SweepResult :type "HitResult Structure (by ref)"))
  ;[1 1 1] Comment
  (bind _ascapsule_collision (cast `CapsuleComponent` OtherComp))
  (if (`ActorComponent.ComponentHasTag` _ascapsule_collision "PlayerCapsule")
    (`/Engine/EditorBlueprintResources/StandardMacros.IsValid` _ascapsule_collision
      (:`Is Valid`
        (if (not (`self.Verrouiller`))
          (`self.1`))))))

(event `1`
  ;[1 1 1] Comment
  (bind (_direction _door1 _door2) (`Timeline|Mover` :!label _label)
    (:`Update`
      (`SceneComponent.K2_SetRelativeLocation` (`self.StaticMesh`) (`KismetMathLibrary.MakeVector` 0.0 _door1) false false)
      (`SceneComponent.K2_SetRelativeLocation` (`self.StaticMesh1`) (`KismetMathLibrary.MakeVector` 0.0 _door2) false false))))

(event `2`
  ;[1 1 1] Comment
  (goto _label :!via `Reverse`))

(event `self.BoxTrigger.OnComponentEndOverlap`
  (params (OverlappedComponent :type "PrimitiveComponent Object Reference") (OtherActor :type "Actor Object Reference") (OtherComp :type "PrimitiveComponent Object Reference") (OtherBodyIndex :type Integer))
  ;[1 1 1] Comment
  (bind _ascapsule_collision (cast `CapsuleComponent` OtherComp))
  (if (`ActorComponent.ComponentHasTag` _ascapsule_collision "PlayerCapsule")
    (`/Engine/EditorBlueprintResources/StandardMacros.IsValid` _ascapsule_collision
      (:`Is Valid`
        (if (not (`self.Verrouiller`))
          (`KismetSystemLibrary.Delay` 1.2)
          (`self.2`))))))

(fn `UserConstructionScript`)