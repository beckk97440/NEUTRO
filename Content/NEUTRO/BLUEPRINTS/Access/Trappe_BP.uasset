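; Trappe_BP is a hatch that swings its Cage open once the padlock referenced by CadenasRef is no longer valid.
; Tick polls that reference and fires OpenCage a single time through a DoOnce.
; OpenCage plays a timeline whose Alpha output directly sets the Cage's relative yaw, with zero pitch and roll.
; BeginPlay stores the Cage's initial world rotation, though the opening logic does not use it.
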(event `self.ReceiveTick`
  (params (DeltaSeconds :type "Float (single-precision)"))
  ;[1 1 1] Comment
  (`/Engine/EditorBlueprintResources/StandardMacros.IsValid` (`self.Cadenas_Ref`)
    (:`Is Not Valid`
      (`/Engine/EditorBlueprintResources/StandardMacros.DoOnce` false
        (:`Completed`
          (`self.OpenCage`))))))

(event `self.ReceiveBeginPlay`
  (set `self.CageInitialRotation` (`SceneComponent.K2_GetComponentRotation` (`self.Cage`))))

(event `OpenCage`
  (bind (_direction _alpha) (`Timeline|Timeline_0`)
    (:`Update`
      (`SceneComponent.K2_SetRelativeRotation` (`self.Cage`) (`KismetMathLibrary.MakeRotator` 0.0 0.0 _alpha) false false))))

(fn `UserConstructionScript`)