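; Door actor that the player can open and close, or that reports itself as closed when locked.
; OpenDoor checks the Verrouiller lock flag, then a FlipFlop alternately plays and reverses the Mover timeline, which drives the mesh's relative yaw.
; When locked, DoorClosed briefly sets a "Seems closed..." thought on the player character, cast to Neutro_ControllerBP.
; The start rotation is saved on BeginPlay but not used in the movement.
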(event `self.ReceiveBeginPlay`
  ;[1 1 1] EventBeginPlay
  (set `self.DoorStartRotation` (`SceneComponent.K2_GetComponentRotation` (`self.StaticMesh`))))

(event `OpenDoor`
  ;[1 1 1] OpenDoorEvent
  (if (`self.Verrouiller`)
    (`self.DoorClosed`)
    (else
      (`/Engine/EditorBlueprintResources/StandardMacros.FlipFlop`
        (:`A`
          (bind (_direction _alpha) (`Timeline|Mover` :!label _label)
            (:`Update`
              (`SceneComponent.K2_SetRelativeRotation` (`self.StaticMesh`) (`KismetMathLibrary.MakeRotator` 0.0 0.0 _alpha) false false))))
        (:`B`
          (goto _label :!via `Reverse`))))))

(event `DoorClosed`
  ;[1 1 1] OpenDoorEvent
  (bind _asneutro_controller_bp (cast `/Game/NEUTRO/BLUEPRINTS/Neutro_ControllerBP` (`GameplayStatics.GetPlayerCharacter` 0)))
  (set `/Game/NEUTRO/BLUEPRINTS/Neutro_ControllerBP.PlayerThinking` "Seems closed..." _asneutro_controller_bp)
  (`KismetSystemLibrary.Delay` 2.0)
  (set `/Game/NEUTRO/BLUEPRINTS/Neutro_ControllerBP.PlayerThinking` "" _asneutro_controller_bp))

(fn `UserConstructionScript`)