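; Physics prop that hurts and alerts patrol NPCs it strikes, with physics simulation switched on or off at BeginPlay by an enum setting.
; On hitting a BP_NPC_Patrol, speed above a threshold applies damage scaled by the prop's matter rate and sends an alert, while slower moving hits only alert.
; Alerts go to the NPC as behavior trigger component messages, with each branch throttled by a delayed DoOnce reset.
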(event `self.ReceiveBeginPlay`
  ;[1 1 1] BeginPlay
  (if (`|EnumEquality` (`self.Physique?`) "NewEnumerator0")
    (`PrimitiveComponent.SetSimulatePhysics` (`self.Props_Matiere_SM`) true)
    (else
      (`PrimitiveComponent.SetSimulatePhysics` (`self.Props_Matiere_SM`) false))))

(event `self.Props_Matiere_SM.OnComponentHit`
  (params (HitComponent :type "PrimitiveComponent Object Reference") (OtherActor :type "Actor Object Reference") (OtherComp :type "PrimitiveComponent Object Reference") (NormalImpulse :type "Vector Structure") (Hit :type "HitResult Structure (by ref)"))
  (bind _returnvalue (`KismetMathLibrary.VSize` (`SceneComponent.GetComponentVelocity` (`self.Props_Matiere_SM`))))
  ;[1 1 1] OnHit
  (bind _output_get (set `self.SetHitActor` OtherActor))
  (if (== (`GameplayStatics.GetObjectClass` _output_get) "/Game/AIBehaviorToolkit/Blueprints/BP_NPC_Patrol.BP_NPC_Patrol_C")
    (bind _asbp_npc_patrol (cast `/Game/AIBehaviorToolkit/Blueprints/BP_NPC_Patrol` (`self.SetHitActor`)))
    (set `self.RefNPCPatrol` _asbp_npc_patrol)
    (if (> _returnvalue 400.0)
      (`/Engine/EditorBlueprintResources/StandardMacros.DoOnce` false :!label _label
        (:`Completed`
          (`GameplayStatics.ApplyDamage` _asbp_npc_patrol (* (`self.PropsTauxMatiere`) 2.0))
          (`self.SendAlert`)
          (`KismetSystemLibrary.Delay` 1.0)
          (goto _label :!via `Reset`)))
      (elif (!= _returnvalue 0.0)
        (`/Engine/EditorBlueprintResources/StandardMacros.DoOnce` false :!label _label_2
          (:`Completed`
            (`self.SendAlert`)
            (`KismetSystemLibrary.Delay` 1.0)
            (goto _label_2 :!via `Reset`)))))))

(event `SendAlert`
  ;[1 1 1] OnHit
  ;;[0.6769 1 0.8881] SendAlertEvent
  (`/Game/AIBehaviorToolkit/Blueprints/BP_BehaviorTriggerComponent.SendDirectMessage` (`self.BP_BehaviorTriggerComponent`) (`self.RefNPCPatrol`) "NewEnumerator3"))

(fn `UserConstructionScript`)